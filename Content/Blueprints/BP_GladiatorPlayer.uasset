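; Player gladiator Blueprint that handles the game's UI: HUD life display, pause menu and game-over screen.
; On BeginPlay it creates the HUD outside the main menu level and binds to the hurt event to update life and check for death.
; At zero life or below, a delayed game-over widget appears and pauses the game.
; Pause and Unpause graphs toggle cursor, input mode and pause state, with keyboard focus set on menu buttons.
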(event Custom|GetHurt
  ;[1 1 1] UI
  (Variables|/Game/Blueprints/UI/HUD.HUD_C|Setlife (stale EventBeginPlay _returnvalue_2) (Variables|Default|Getlife)))

(event Custom|GameOver
  ;[1 1 1] UI
  (Math|Integer|CompareInt (Variables|Default|Getlife)
    (:==
      _)
    (:<
      _))
  (Utilities|FlowControl|Delay 2.0)
  (bind _returnvalue (UserInterface|CreateWidget "/Game/Blueprints/UI/GameOver.GameOver_C"))
  (UserInterface|Viewport|AddtoViewport _returnvalue 0)
  (Variables|/Script/Engine.PlayerController|SetbShowMouseCursor (Game|GetPlayerController 0) true)
  (Utilities|FlowControl|Delay 0.1)
  (Widget|SetKeyboardFocus (Variables|/Game/Blueprints/UI/GameOver.GameOver_C|GetRetry _returnvalue))
  (Game|SetGamePaused true))

(event EventBeginPlay
  ;[1 1 1] UI
  (Utilities|FlowControl|Sequence
    (:then_0
      (bind _returnvalue (Game|GetCurrentLevelName true))
      (if (not (Utilities|Enum|Equal(Enum) _returnvalue "MainMenuLVL"))
        (bind _returnvalue_2 (UserInterface|CreateWidget "/Game/Blueprints/UI/HUD.HUD_C"))
        (UserInterface|Viewport|AddtoViewport _returnvalue_2 0)
        (Variables|/Game/Blueprints/UI/HUD.HUD_C|Setlife _returnvalue_2 (Variables|Default|GetmaxLife))
        (Variables|/Game/Blueprints/UI/HUD.HUD_C|SetmaxLife _returnvalue_2 (Variables|Default|GetmaxLife))
        (EventDispatchers|BindEventtoHurtEvent (delegate Custom|GetHurt))))
    (:then_1
      (EventDispatchers|BindEventtoHurtEvent (delegate Custom|GameOver)))))

(event Input|ActionEvents|InputActionPause
  (params (Key :type Key%20Structure :default "None"))
  (bind _returnvalue (Game|GetPlayerController 0))
  ;[1 1 1] Pause / Unpause
  (:Pressed
    (Utilities|IsValid (Variables|Default|GetPauseMenu%20REF)
      (:Is%20Valid
        _)
      (:Is%20Not%20Valid
        (bind _returnvalue_2 (UserInterface|CreateWidget "/Game/Blueprints/UI/Pause.Pause_C"))
        (Variables|Default|SetPauseMenu%20REF _returnvalue_2)))
    (if (Game|IsGamePaused)
      (|Unpause (Variables|Default|GetPauseMenu%20REF) _returnvalue)
      (else
        (Sequencer|Player|Pause (Variables|Default|GetPauseMenu%20REF) _returnvalue)))))

(fn ConstructionScript)