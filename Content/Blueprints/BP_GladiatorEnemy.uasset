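; BP_GladiatorEnemy is an enemy character with a world widget life bar and a death animation.
; On BeginPlay outside the main menu level, it hides the bar, seeds it with MaxLife after a short delay, and binds to hurt, lock and unlock events.
; Hurt updates the bar and plays the death montage at zero life.
; Lock and unlock events show and hide the bar.
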(event Custom|HideWidget
  (Development|SetHiddeninGame (Variables|Default|GetLifeBar) true false))

(event Custom|DisplayWidget
  (Development|SetHiddeninGame (Variables|Default|GetLifeBar) false false))

(event Custom|GetHurt
  (Variables|/Game/Blueprints/UI/EnemiesLifeBar.EnemiesLifeBar_C|Setlife (stale EventBeginPlay _asenemies_life_bar) (Variables|Default|Getlife))
  (if (<= (Variables|Default|Getlife) 0)
    (Animation|Montage|PlayMontage (Variables|Character|GetMesh) "/Game/Characters/DwarfGrunt/Anims/Death2_Montage.Death2_Montage")))

(event EventBeginPlay
  (bind _lifebar (Variables|Default|GetLifeBar))
  (bind _returnvalue (Game|GetCurrentLevelName true))
  (if (not (Utilities|Enum|Equal(Enum) _returnvalue "MainMenuLVL"))
    (Utilities|FlowControl|Sequence
      (:then_0
        (Utilities|FlowControl|Delay 0.04)
        (Development|SetHiddeninGame _lifebar true false)
        (bind _asenemies_life_bar (Utilities|Casting|CastToEnemiesLifeBar (UserInterface|GetUserWidgetObject _lifebar)))
        (Variables|/Game/Blueprints/UI/EnemiesLifeBar.EnemiesLifeBar_C|Setlife _asenemies_life_bar (Variables|Default|GetmaxLife))
        (Variables|/Game/Blueprints/UI/EnemiesLifeBar.EnemiesLifeBar_C|SetmaxLife _asenemies_life_bar (Variables|Default|GetmaxLife))
        (EventDispatchers|BindEventtoHurtEvent (delegate Custom|GetHurt)))
      (:then_1
        (EventDispatchers|BindEventtoUnlockEvent (delegate Custom|HideWidget))
        (EventDispatchers|BindEventtoLockEvent (delegate Custom|DisplayWidget))))))

(fn ConstructionScript)