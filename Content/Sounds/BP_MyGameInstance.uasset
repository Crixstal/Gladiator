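; Game instance Blueprint, going by its name, that switches between day (Coliseum_Cue) and night (Night_Cue) audio.
; Each function stops the shared Audio component if valid, then creates and stores a new 2D sound at the given volume.
; Playback starts at a random whole-minute offset within the first half hour.
; Only the day function exposes persistence across level transitions.
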(fn PlayAudioDay
  (params (Volume :type Float%20%28single-precision%29) (bPersistAcrossLevelTransition :type Boolean))
  (Utilities|IsValid (Variables|Default|Getaudio)
    (:Is%20Valid
      (Audio|Components|Audio|Stop (Variables|Default|Getaudio)))
    (:Is%20Not%20Valid
      _))
  (bind _returnvalue (Audio|CreateSound2D "/Game/Sounds/Coliseum_Cue.Coliseum_Cue" Volume 1.0 0.0 0 bPersistAcrossLevelTransition))
  (bind _output_get (Variables|Default|Setaudio _returnvalue))
  (Audio|Components|Audio|Play _output_get (Math|Conversions|ToFloat(Integer) (* (Math|Random|RandomInteger 31) 60))))

(fn PlayAudioNight
  (params (Volume :type Float%20%28single-precision%29))
  (Utilities|IsValid (Variables|Default|Getaudio)
    (:Is%20Valid
      (Audio|Components|Audio|Stop (Variables|Default|Getaudio)))
    (:Is%20Not%20Valid
      _))
  (bind _returnvalue (Audio|CreateSound2D "/Game/Sounds/NightAmbiance/Night_Cue.Night_Cue" Volume 1.0 0.0 0))
  (bind _output_get (Variables|Default|Setaudio _returnvalue))
  (Audio|Components|Audio|Play _output_get (Math|Conversions|ToFloat(Integer) (* (Math|Random|RandomInteger 31) 60))))